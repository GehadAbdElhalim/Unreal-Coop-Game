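; BP_Grenade is a timed grenade actor that explodes after a delay from BeginPlay, then destroys itself.
; On detonation it spawns an explosion particle effect and loops over components overlapping its ExplosionSphere.
; Each physics-simulating component receives a constant-falloff radial force as an acceleration change.
; Full radial damage across the sphere radius is applied inside that same loop, so it repeats once per simulating component.
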(event EventBeginPlay
  (Utilities|FlowControl|Delay (Variables|Default|GetTimer))
  (Effects|SpawnEmitteratLocation "/Game/WeaponEffects/Explosion/P_Explosion.P_Explosion" (Transformation|GetActorLocation))
  (for _array_element (Class|PrimitiveComponent|GetOverlappingComponents (Variables|Default|GetExplosion%20Sphere))
    (if (Physics|IsSimulatingPhysics _array_element "None")
      (Physics|AddRadialForce _array_element (Transformation|GetActorLocation) (Variables|/Script/Engine.SphereComponent|GetSphereRadius (Variables|Default|GetExplosion%20Sphere)) (Variables|Default|GetForce) "RIF_Constant" true)
      (Game|Damage|ApplyRadialDamage (Variables|Default|GetDamage) (Transformation|GetActorLocation) (Variables|/Script/Engine.SphereComponent|GetSphereRadius (Variables|Default|GetExplosion%20Sphere)) 0 0 self (Game|GetInstigatorController) true "ECC_Visibility")))
  (Actor|DestroyActor))

(fn ConstructionScript)